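; Elemental ability area actor that blocks as ice, slows characters as water, heals as steam or damages as fire.
; A multicast event sets collision, type-specific particles and a persistence-based lifespan, with ice also scaling by level.
; Overlaps track characters; Tick applies level-scaled damage or negative-damage healing every second through HealthComponent.
; Water reduces MaxWalkSpeed and restores it on exit using one AbilityModifier shared by all characters.
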(event `self.ReceiveBeginPlay`)

(event `self.ReceiveTick`
  (params (DeltaSeconds :type "Float (single-precision)"))
  ;[0.9401 0.7186 1] Trigger damage or heal every second
  (if (`self.bTriggerStayAbility`)
    (bind _output_get (set `self.TimeTillNextTrigger` (- (`self.TimeTillNextTrigger`) DeltaSeconds)))
    (if (<= _output_get 0.0)
      (set `self.TimeTillNextTrigger` 1.0)
      ;[0.933 0.6554 1] Deal damage or heal characters in the fire or steam overlap
      (for _array_element (`self.CharacterArray`)
        (bind _returnvalue (`self.GetComponentByClass` _array_element "/Script/AdvGamesProgramming.HealthComponent"))
        (`HealthComponent.OnTakeDamage` _returnvalue (`self.AbilityModifier`))
        (cast `/Game/Blueprints/PlayerCharacterBlueprint` _array_element
          (:`then`
            (bind _returnvalue_2 (`KismetStringLibrary.Conv_DoubleToString` (`HealthComponent.CurrentHealth` _returnvalue)))
            (`KismetSystemLibrary.PrintString` (`KismetStringLibrary.Concat_StrStr` "Player Health Remaining: " _returnvalue_2) true false (struct :`R` 1.0 :`A` 1.0)))
          (:`CastFailed`
            (`KismetSystemLibrary.PrintString` (`KismetStringLibrary.Concat_StrStr` "Enemy Health Remaining:" _returnvalue_2) true false (struct :`R` 0.019269 :`G` 1.0 :`A` 1.0))))))))

(event `MulticastSetMaterial`
  (`self.SetAreaMaterial`))

(event `DisableParticles`
  (params (ParticleSystem :type "ParticleSystemComponent Object Reference") (WaitTime :type "Float (double-precision)"))
  ;[0.9922 0.5137 1] Turn off particles after their lifespan
  (`KismetSystemLibrary.Delay` WaitTime)
  (`ActorComponent.SetActive` ParticleSystem false false)
  (`KismetSystemLibrary.Delay` 0.5)
  (`ActorComponent.K2_DestroyComponent` ParticleSystem))

(event `self.ReceiveActorBeginOverlap`
  (params (OtherActor :type "Actor Object Reference"))
  ;[0.9922 0.5137 1] Set off on overlap events
  (bind _ascharacter (cast `Character` OtherActor))
  (`KismetArrayLibrary.Array_Add` (`self.CharacterArray`) _ascharacter)
  (switch `AbilityType` (`self.CurrentAbilityType`)
    (:`WATER`
      (`self.WaterTrigger` (`Character.CharacterMovement` _ascharacter)))
    (:`STEAM`
      (`self.SteamTrigger`))
    (:`FIRE`
      (`self.FireTrigger`))))

(event `self.ReceiveActorEndOverlap`
  (params (OtherActor :type "Actor Object Reference"))
  ;[1 0.6515 0.9708] Remove characters upon leaving the overlap
  (bind _ascharacter (cast `Character` OtherActor))
  (`self.ExitWaterTrigger` (`Character.CharacterMovement` _ascharacter))
  (`KismetArrayLibrary.Array_RemoveItem` (`self.CharacterArray`) _ascharacter)
  (if (<= (`KismetArrayLibrary.Array_Length` (`self.CharacterArray`)) 0)
    (set `self.bTriggerStayAbility` false)
    (set `self.TimeTillNextTrigger` 0.0)))

(fn `ExitWaterTrigger`
  (params (CharacterMovement :type "CharacterMovementComponent Object Reference"))
  (switch `AbilityType` (`self.CurrentAbilityType`)
    (:`WATER`
      (set `CharacterMovementComponent.MaxWalkSpeed` (+ (`CharacterMovementComponent.MaxWalkSpeed` CharacterMovement) (`self.AbilityModifier`)) CharacterMovement))))

(fn `FireTrigger`
  (set `self.bTriggerStayAbility` true)
  (set `self.AbilityModifier` (* (`self.AbilityLevel`) 3.0)))

(fn `SetAreaMaterial`
  (bind _cube (`self.Cube`))
  (bind _bisice (`self.SetParticles` (`self.CurrentAbilityType`)))
  (if _bisice
    (`PrimitiveComponent.SetMaterial` (`self.Cube`) 0 "/Game/Materials/AbilityAreaMaterials/IceMaterial.IceMaterial")
    ;[0.9004 0.4604 1] Set to overlap or collision based on ability type
    (`PrimitiveComponent.SetCollisionResponseToAllChannels` _cube "ECR_Block")
    ;[1 0.448 0.9539] Set object lifespan based on ability persistence (and level if it's ice)
    (`self.SetLifeSpan` (/ (* (`self.AbilityLevel`) (`self.AbilityPersistence`)) 5.0))
    (else
      (`PrimitiveComponent.SetCollisionResponseToAllChannels` _cube "ECR_Overlap")
      (`self.SetLifeSpan` (`self.AbilityPersistence`)))))

(fn `SetParticles`
  (params (AbilityType :type "AbilityType Enum" :default "ICE"))
  (returns (bIsIce :type Boolean))
  (bind _returnvalue (`self.K2_GetActorLocation`))
  (bind _abilitypersistence (`self.AbilityPersistence`))
  (switch `AbilityType` AbilityType
    (:`ICE`
      (`GameplayStatics.SpawnEmitterAtLocation` "/Game/MyParticleSystems/Ice/P_Ice.P_Ice" _returnvalue)
      (return true))
    (:`WATER`
      (bind _returnvalue_2 (`GameplayStatics.SpawnEmitterAtLocation` "/Game/MyParticleSystems/Water/p_water_GPU.p_water_GPU" _returnvalue (struct) (1.0 1.0 1.0) false))
      (`self.DisableParticles` _returnvalue_2 _abilitypersistence))
    (:`STEAM`
      (bind _returnvalue_3 (`GameplayStatics.SpawnEmitterAtLocation` "/Game/MyParticleSystems/Steam/P_Steam.P_Steam" _returnvalue (struct) (1.0 1.0 1.0) false))
      (`self.DisableParticles` _returnvalue_3 _abilitypersistence))
    (:`FIRE`
      (bind _returnvalue_4 (`GameplayStatics.SpawnEmitterAtLocation` "/Game/MyParticleSystems/Fire/P_Fire.P_Fire" _returnvalue (struct) (1.0 1.0 1.0) false))
      (`self.DisableParticles` _returnvalue_4 _abilitypersistence)))
  (return false))

(fn `SteamTrigger`
  (set `self.bTriggerStayAbility` true)
  (set `self.AbilityModifier` (* (`self.AbilityLevel`) -1.0)))

(fn `UserConstructionScript`)

(fn `WaterTrigger`
  (params (CharacterMovement :type "CharacterMovementComponent Object Reference"))
  (bind _maxwalkspeed (`CharacterMovementComponent.MaxWalkSpeed` CharacterMovement))
  (bind _output_get (set `self.AbilityModifier` (/ (* (`self.AbilityLevel`) _maxwalkspeed) 10.0)))
  (set `CharacterMovementComponent.MaxWalkSpeed` (- _maxwalkspeed _output_get) CharacterMovement))