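; EnemyCharacterBlueprint is an enemy character that fires a gun and can play a death animation.
; Its Fire event casts the Gun child actor to GunBlueprint and fires along the given direction plus a random unit-vector offset scaled by TargetAccuracyOffset.
; It then rotates the enemy to face the unperturbed direction, so inaccuracy affects only the shot.
; A separate PlayDeathAnimation event plays Death_1 once on the mesh.
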(event `self.Fire`
  (params (FireDirection :type "Vector Structure"))
  (bind _asgun_blueprint (cast `/Game/Blueprints/GunBlueprint` (`ChildActorComponent.ChildActor` (`self.Gun`))))
  (`/Game/Blueprints/GunBlueprint.Fire` _asgun_blueprint (+ (* (`KismetMathLibrary.RandomUnitVector`) (`self.TargetAccuracyOffset`)) FireDirection))
  (`self.K2_SetActorRotation` (`KismetMathLibrary.Conv_VectorToRotator` FireDirection)))

(event `self.PlayDeathAnimation`
  (`SkeletalMeshComponent.PlayAnimation` (`self.Mesh`) "/Game/Assets/Mannequin/AnimStarterPack/Death_1.Death_1" false))

(fn `UserConstructionScript`)